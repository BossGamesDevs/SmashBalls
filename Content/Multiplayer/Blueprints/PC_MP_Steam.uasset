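; Player controller for Steam multiplayer that handles the quit menu and respawn requests.
; M flip-flops a newly created W_QuitGame widget on and off screen, switching input mode and mouse cursor with it.
; P, when no valid pawn is controlled, calls a server-named event that asks GM_MP_Steam to respawn this controller through ServerRespawnPlayer1.
; An older respawn path, marked broken, remains with its caller disconnected.
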(event `Key|M`
  (params (Key :type "Key Structure"))
  (bind _returnvalue (`GameplayStatics.GetPlayerController` 0))
  ;[1 1 1] Quit Game Toggles Quit Game Menu
  (:`Pressed`
    (`/Engine/EditorBlueprintResources/StandardMacros.FlipFlop`
      (:`A`
        (bind _returnvalue_2 (`|CreateWidget` "/Game/Multiplayer/Widgets/W_QuitGame.W_QuitGame_C" _returnvalue))
        (`UserWidget.AddToViewport` _returnvalue_2 0)
        (`WidgetBlueprintLibrary.SetInputMode_GameAndUIEx` _returnvalue _returnvalue_2)
        (set `PlayerController.bShowMouseCursor` true _returnvalue))
      (:`B`
        (`Widget.RemoveFromParent` _returnvalue_2)
        (`WidgetBlueprintLibrary.SetInputMode_GameOnly` _returnvalue)
        (set `PlayerController.bShowMouseCursor` false _returnvalue)))))

(event `Key|P`
  (params (Key :type "Key Structure"))
  ;[0 0 0] BROKED
)

(event `Server_RequestRespawn`
  (bind _returnvalue (`GameplayStatics.GetGameMode`))
  ;[0 0 0] BROKED
  (`/Engine/EditorBlueprintResources/StandardMacros.IsValid` _returnvalue
    (:`Is Valid`
      (bind _asgm_mp_steam (cast `/Game/Multiplayer/Blueprints/GM_MP_Steam` _returnvalue))
      (`/Engine/EditorBlueprintResources/StandardMacros.IsValid` _asgm_mp_steam
        (:`Is Valid`
          (`/Game/Multiplayer/Blueprints/GM_MP_Steam.Server_RespawnPlayer` _asgm_mp_steam self))))))

(event `Key|P`
  (params (Key :type "Key Structure"))
  (:`Pressed`
    (`/Engine/EditorBlueprintResources/StandardMacros.IsValid` (`self.K2_GetPawn` self)
      (:`Is Not Valid`
        (`self.Server_RequestRespawn1`)))))

(event `Server_RequestRespawn1`
  (bind _returnvalue (`GameplayStatics.GetGameMode`))
  (`/Engine/EditorBlueprintResources/StandardMacros.IsValid` _returnvalue
    (:`Is Valid`
      (bind _asgm_mp_steam (cast `/Game/Multiplayer/Blueprints/GM_MP_Steam` _returnvalue))
      (`/Engine/EditorBlueprintResources/StandardMacros.IsValid` _asgm_mp_steam
        (:`Is Valid`
          (`/Game/Multiplayer/Blueprints/GM_MP_Steam.Server_RespawnPlayer1` _asgm_mp_steam self))))))

(fn `UserConstructionScript`)