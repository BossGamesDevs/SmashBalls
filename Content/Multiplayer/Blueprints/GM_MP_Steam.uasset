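; Multiplayer game mode that respawns players and starts timed enemy spawning.
; BeginPlay caches all PlayerStarts in SpawnPoints1, then sets a looping timer calling SpawnEnemy on the first EnemySpawner_BP at EnemiesPerSecond.
; Server_RespawnPlayer1 spawns and possesses a BP_Character_Master, rolling location and rotation from separate random PlayerStart picks.
; Server_RespawnPlayer, marked broken, duplicates this using SpawnPoints, whose setup never runs.
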(event `self.ReceiveBeginPlay`
  ;[1 1 1] GOOD ONE
  (bind _outactors (`GameplayStatics.GetAllActorsOfClass` "/Script/Engine.PlayerStart"))
  (set `self.SpawnPoints1` _outactors)
  (`self.SpawnEnemies`))

(event `Server_RespawnPlayer1`
  (params (PlayerController :type "PlayerController Object Reference"))
  (bind _spawnpoints1 (`self.SpawnPoints1`))
  (bind (_returnvalue_location _returnvalue_rotation) (`KismetMathLibrary.BreakTransform` (`self.GetTransform` (`|GetArrayItem` _spawnpoints1 (`KismetMathLibrary.RandomIntegerInRange` 0 (- (`KismetArrayLibrary.Array_Length` _spawnpoints1) 1))))))
  ;[1 1 1] GOOD ONE
  (`/Engine/EditorBlueprintResources/StandardMacros.IsValid` PlayerController
    (:`Is Valid`
      (bind _returnvalue (`|SpawnActorFromClass` "/Game/SmashBallsGame/Characters/Blueprints/BP_Character_Master.BP_Character_Master_C" (`KismetMathLibrary.MakeTransform` _returnvalue_location _returnvalue_rotation) "AlwaysSpawn" "OverrideRootScale" null null))
      (`/Engine/EditorBlueprintResources/StandardMacros.IsValid` _returnvalue
        (:`Is Valid`
          (`Controller.Possess` PlayerController _returnvalue))))))

(event `SpawnEnemies`
  ;[1 1 1] SpawnEnemies
  (bind _outactors (`GameplayStatics.GetAllActorsOfClass` "/Game/SmashBallsGame/Characters/Blueprints/EnemySpawner_BP.EnemySpawner_BP_C"))
  (bind _output_get (set `self.EnemySpawnerRef` (`|GetArrayItem` _outactors)))
  (`KismetSystemLibrary.K2_SetTimer` _output_get "SpawnEnemy" (/ 1.0 (`self.EnemiesPerSecond`)) true))

(event `Server_RespawnPlayer`
  (params (PlayerController :type "PlayerController Object Reference"))
  (bind _spawnpoints (`self.SpawnPoints`))
  (bind (_returnvalue_location _returnvalue_rotation) (`KismetMathLibrary.BreakTransform` (`self.GetTransform` (`|GetArrayItem` _spawnpoints (`KismetMathLibrary.RandomIntegerInRange` 0 (- (`KismetArrayLibrary.Array_Length` _spawnpoints) 1))))))
  ;[0 0 0] BROKEN
  (`/Engine/EditorBlueprintResources/StandardMacros.IsValid` PlayerController
    (:`Is Valid`
      (bind _returnvalue (`|SpawnActorFromClass` "/Game/SmashBallsGame/Characters/Blueprints/BP_Character_Master.BP_Character_Master_C" (`KismetMathLibrary.MakeTransform` _returnvalue_location _returnvalue_rotation) "AlwaysSpawn" "OverrideRootScale" null null))
      (`/Engine/EditorBlueprintResources/StandardMacros.IsValid` _returnvalue
        (:`Is Valid`
          (`Controller.Possess` PlayerController _returnvalue))))))

(fn `UserConstructionScript`)