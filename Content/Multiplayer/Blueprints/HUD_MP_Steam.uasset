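; HUD Blueprint for the Steam multiplayer setup that puts the W_Container widget on screen.
; On BeginPlay it creates that widget for the owning player controller and adds it to the viewport.
; DrawHUD does nothing; a centered default-crosshair texture draw is left disconnected and never runs.
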(event `self.ReceiveBeginPlay`
  (bind _returnvalue (`|CreateWidget` "/Game/Multiplayer/Widgets/W_Container.W_Container_C" (`self.GetOwningPlayerController`)))
  (`UserWidget.AddToViewport` _returnvalue 0))

(event `self.ReceiveDrawHUD`
  (params (SizeX :type Integer) (SizeY :type Integer)))

(fn `UserConstructionScript`)