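; Master pickup actor that gives overlapping player characters either health or ammo, depending on its pickup type.
; Collision overlap calls a server event that adds the clamped amount to health or the current weapon's ammo reserve, only if below maximum.
; On success it multicasts a sound, hides itself and disables collision, then reappears after a respawn timer.
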(event `self.PickupCollision.OnComponentBeginOverlap`
  (params (OverlappedComponent :type "PrimitiveComponent Object Reference") (OtherActor :type "Actor Object Reference") (OtherComp :type "PrimitiveComponent Object Reference") (OtherBodyIndex :type Integer) (bFromSweep :type Boolean) (SweepResult :type "HitResult Structure (by ref)"))
  (bind _asbp_character_master (cast `/Game/SmashBallsGame/Characters/Blueprints/BP_Character_Master` OtherActor))
  (`self.Server_OnOverlap` _asbp_character_master))

(event `Server_OnOverlap`
  (params (Character :type "/Game/SmashBallsGame/Characters/Blueprints/BP_Character_Master Object Reference"))
  (bind _pickupcollision (`self.PickupCollision`))
  (bind _pickupcollision_2 (`self.PickupCollision`))
  (bind _currenthealth (`/Game/SmashBallsGame/Characters/Blueprints/BP_Character_Master.CurrentHealth` Character))
  (bind _maxhealth (`/Game/SmashBallsGame/Characters/Blueprints/BP_Character_Master.MaxHealth` Character))
  (bind _bpcurrentweaponref (`/Game/SmashBallsGame/Characters/Blueprints/BP_Character_Master.BPCurrentWeaponRef` Character))
  (bind _currentmaxammo (`/Game/SmashBallsGame/Weapons/Blueprints/BP_Weapon_Master.CurrentMaxAmmo` _bpcurrentweaponref))
  (bind _maxammo (`/Game/SmashBallsGame/Weapons/Blueprints/BP_Weapon_Master.MaxAmmo` _bpcurrentweaponref))
  (switch `/Game/SmashBallsGame/GamePlay/Blueprints/E_Pickup_Types` (`self.PickupType`)
    (:`NewEnumerator0`
      ;[1 1 1] Health Pickup
      (if (< _currenthealth _maxhealth)
        (set `/Game/SmashBallsGame/Characters/Blueprints/BP_Character_Master.CurrentHealth` (`KismetMathLibrary.Clamp` (+ (`self.HealthAmountToGive`) _currenthealth) 0 _maxhealth) Character)
        (`self.Multicast_PickupSound`)
        (`self.SetActorHiddenInGame` true)
        (`PrimitiveComponent.SetCollisionEnabled` _pickupcollision "NoCollision")
        (`KismetSystemLibrary.Delay` (`self.RespawnTimer`))
        (`PrimitiveComponent.SetCollisionEnabled` _pickupcollision "QueryOnly")
        (`self.SetActorHiddenInGame` false)))
    (:`NewEnumerator1`
      ;[1 1 1] Ammo Pickup
      (if (< _currentmaxammo _maxammo)
        (set `/Game/SmashBallsGame/Weapons/Blueprints/BP_Weapon_Master.CurrentMaxAmmo` (`KismetMathLibrary.Clamp` (+ (`self.AmmoAmountToGive`) _currentmaxammo) 0 _maxammo) _bpcurrentweaponref)
        (`self.Multicast_PickupSound`)
        (`self.SetActorHiddenInGame` true)
        (`PrimitiveComponent.SetCollisionEnabled` _pickupcollision_2 "NoCollision")
        (`KismetSystemLibrary.Delay` (`self.RespawnTimer`))
        (`PrimitiveComponent.SetCollisionEnabled` _pickupcollision_2 "QueryOnly")
        (`self.SetActorHiddenInGame` false)))))

(event `Multicast_PickupSound`
  ;[1 1 1] Multicast Pickup Sound
  (`GameplayStatics.PlaySoundAtLocation` (`self.PickupSound`) (`self.K2_GetActorLocation`)))

(fn `UserConstructionScript`)