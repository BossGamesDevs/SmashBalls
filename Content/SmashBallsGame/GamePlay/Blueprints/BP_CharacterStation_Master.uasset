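; BP_CharacterStation_Master is a station actor where a player standing in its trigger box can switch between light, medium and heavy characters.
; Overlap by a BP_Character_Master with a PC_MP_Steam controller enables input on the station, and leaving disables it.
; Keys 1, 2 and 3 call the matching ServerSelect function on the character cached from the overlap cast, passing its controller.
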(event `self.TriggerBox.OnComponentBeginOverlap`
  (params (OverlappedComponent :type "PrimitiveComponent Object Reference") (OtherActor :type "Actor Object Reference") (OtherComp :type "PrimitiveComponent Object Reference") (OtherBodyIndex :type Integer) (bFromSweep :type Boolean) (SweepResult :type "HitResult Structure (by ref)"))
  (bind _asbp_character_master (cast `/Game/SmashBallsGame/Characters/Blueprints/BP_Character_Master` OtherActor))
  (bind _aspc_mp_steam (cast `/Game/Multiplayer/Blueprints/PC_MP_Steam` (`Pawn.GetController` _asbp_character_master)))
  (`self.EnableInput` _aspc_mp_steam))

(event `self.TriggerBox.OnComponentEndOverlap`
  (params (OverlappedComponent :type "PrimitiveComponent Object Reference") (OtherActor :type "Actor Object Reference") (OtherComp :type "PrimitiveComponent Object Reference") (OtherBodyIndex :type Integer))
  (bind _asbp_character_master (cast `/Game/SmashBallsGame/Characters/Blueprints/BP_Character_Master` OtherActor))
  (bind _aspc_mp_steam (cast `/Game/Multiplayer/Blueprints/PC_MP_Steam` (`Pawn.GetController` _asbp_character_master)))
  (`self.DisableInput` _aspc_mp_steam))

(event `Key|One`
  (params (Key :type "Key Structure"))
  (:`Pressed`
    (`/Game/SmashBallsGame/Characters/Blueprints/BP_Character_Master.Server_SelectLightCharacter` (stale `self.TriggerBox.OnComponentBeginOverlap` _asbp_character_master) (`Pawn.GetController` (stale `self.TriggerBox.OnComponentBeginOverlap` _asbp_character_master)))))

(event `Key|Two`
  (params (Key :type "Key Structure"))
  (:`Pressed`
    (`/Game/SmashBallsGame/Characters/Blueprints/BP_Character_Master.Server_SelectMediumCharacter` (stale `self.TriggerBox.OnComponentBeginOverlap` _asbp_character_master) (`Pawn.GetController` (stale `self.TriggerBox.OnComponentBeginOverlap` _asbp_character_master)))))

(event `Key|Three`
  (params (Key :type "Key Structure"))
  (:`Pressed`
    (`/Game/SmashBallsGame/Characters/Blueprints/BP_Character_Master.Server_SelectHeavyCharacter` (stale `self.TriggerBox.OnComponentBeginOverlap` _asbp_character_master) (`Pawn.GetController` (stale `self.TriggerBox.OnComponentBeginOverlap` _asbp_character_master)))))

(fn `UserConstructionScript`)