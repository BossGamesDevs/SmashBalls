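; Base projectile for SmashBallsGame with configurable bouncing, explosive and sticky behavior, ignoring its instigator on collision.
; Hit, stop and bounce events route through server events, with multicasts playing surface-based impact, explosion and bounce effects.
; Non-bouncing projectiles resolve on hit, with sticky explosives attaching to character bones until a timer expires.
; Non-sticky stops share the explosion path, which applies point or radial damage by DamageType, then destroys the actor.
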(event `self.ReceiveBeginPlay`
  ;[0.8632 0.4092 0] EventBeginPlay
  (`PrimitiveComponent.IgnoreActorWhenMoving` (`self.ProjectileCollision`) (`self.GetInstigator`) true)
  (if (`self.IsShouldBounce?`)
    (set `ProjectileMovementComponent.bShouldBounce` true (`self.ProjectileMovement`))))

(event `Server_OnEventHit`
  (params (HitResult :type "HitResult Structure"))
  (bind (_bblockinghit _binitialoverlap _time _distance _location _impactpoint _normal _impactnormal _physmat _hitactor _hitcomponent _hitbonename) (`GameplayStatics.BreakHitResult` HitResult))
  (if (not (`self.IsShouldBounce?`))
    (if (not (`self.IsExplosive?`))
      (`self.Multicast_OnEventHit` HitResult)
      (else
        ;[1 1 1] Sticky Attach Projectile To Character
        (if (`self.IsSticky?`)
          (bind _asbp_character_master (cast `/Game/SmashBallsGame/Characters/Blueprints/BP_Character_Master` _hitactor)
            (:`then`
              (`self.K2_AttachToComponent` (`Character.Mesh` _asbp_character_master) _hitbonename "KeepWorld" "KeepWorld" "KeepWorld"))
            (:`CastFailed`
              _))
          (`KismetSystemLibrary.Delay` (`self.StickyTimer`)))
        ;[1 1 1] Multicast OnProjectileStop
        (`self.Multicast_OnStop` :!label _label)))
    ;[1 1 1] Delect Damage Type
    (switch `/Game/SmashBallsGame/Weapons/Blueprints/E_DamageTypes` (`self.DamageType`)
      (:`NewEnumerator0`
        ;[1 1 1] Deal Normal Bullet Damage
        (`GameplayStatics.ApplyDamage` _hitactor (`KismetMathLibrary.Conv_IntToDouble` (`self.Damage`)) (`self.GetInstigatorController`) self))
      (:`NewEnumerator1`
        ;[1 1 1] Deal Area Of effect Damage
        (`GameplayStatics.ApplyRadialDamage` :`BaseDamage` (`KismetMathLibrary.Conv_IntToDouble` (`self.Damage`)) :`Origin` (`SceneComponent.K2_GetComponentLocation` (`self.ProjectileCollision`)) :`DamageRadius` (`self.DamageRadius`) :`DamageCauser` self :`InstigatedByController` (`self.GetInstigatorController`))))
    ;[1 1 1] Destroy Projectile
    (`self.K2_DestroyActor`)))

(event `self.ReceiveHit`
  (params (MyComp :type "PrimitiveComponent Object Reference") (Other :type "Actor Object Reference") (OtherComp :type "PrimitiveComponent Object Reference") (bSelfMoved :type Boolean) (HitLocation :type "Vector Structure") (HitNormal :type "Vector Structure") (NormalImpulse :type "Vector Structure") (Hit :type "HitResult Structure (by ref)"))
  ;[1 1 1] OnEventHit
  (`self.Server_OnEventHit` Hit))

(event `Multicast_OnEventHit`
  (params (HitResult :type "HitResult Structure"))
  (bind (_bblockinghit _binitialoverlap _time _distance _location _impactpoint _normal _impactnormal _physmat) (`GameplayStatics.BreakHitResult` HitResult))
  (bind _surfacetype (`PhysicalMaterial.SurfaceType` _physmat))
  ;[1 1 1] Impact Effects
  (`GameplayStatics.PlaySoundAtLocation` (select `EPhysicalSurface` _surfacetype :`SurfaceType_Default` (`self.DefaultBulletImpactSound`) :`SurfaceType1` (`self.PlayerBulletImpactSound`) :!type "SoundBase Object Reference") _impactpoint)
  (`GameplayStatics.SpawnEmitterAtLocation` (select `EPhysicalSurface` _surfacetype :`SurfaceType_Default` (`self.DefaultBulletImpactPS`) :`SurfaceType1` (`self.PlayerBulletImpactPS`)) _impactpoint (`KismetMathLibrary.MakeRotFromZ` _impactnormal)))

(event `self.ProjectileMovement.OnProjectileStop`
  (params (ImpactResult :type "HitResult Structure (by ref)"))
  ;[1 1 1] OnProjectileStop
  (`self.Server_OnStop`))

(event `Server_OnStop`
  ;[1 1 1] OnProjectileStop
  (if (not (`self.IsSticky?`))
    (goto _label)))

(event `Multicast_OnStop`
  (bind _projectilecollision (`self.ProjectileCollision`))
  (bind _returnvalue (`SceneComponent.K2_GetComponentLocation` _projectilecollision))
  ;[1 1 1] Explosion Effects
  (`GameplayStatics.PlaySoundAtLocation` (`self.ExplosionSound`) _returnvalue)
  (`GameplayStatics.SpawnEmitterAtLocation` (`self.ExplosionPS`) _returnvalue (`SceneComponent.K2_GetComponentRotation` _projectilecollision)))

(event `self.ProjectileMovement.OnProjectileBounce`
  (params (ImpactResult :type "HitResult Structure (by ref)") (ImpactVelocity :type "Vector Structure (by ref)"))
  ;[1 1 1] OnProjectileBounce
  (`self.Server_OnBounce`))

(event `Server_OnBounce`
  ;[1 1 1] OnProjectileBounce
  (`self.Multicast_OnBounce`))

(event `Multicast_OnBounce`
  ;[1 1 1] OnProjectileBounce
  (`GameplayStatics.PlaySoundAtLocation` "/Game/Assets/Weapons/Audio/Weapons/BulletImpacts/Rifle/Cues/A_Wep_BulletImpact_Rifle_Cue.A_Wep_BulletImpact_Rifle_Cue" (`self.K2_GetActorLocation`)))

(fn `UserConstructionScript`)