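; Enemy character that walks or runs and throws Hadouken projectiles, driven alongside an Enemy_C AI controller.
; The Hadouken montage tells the controller to stop rotating to the player when it completes; spawning launches a forward projectile at a randomly high or low height.
; Health is set on the server at BeginPlay; damage reduces it, and at zero the enemy plays a multicast death sound and is destroyed.
; Pawn sensing only prints the seen pawn's location.
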(event `Walk`
  ;[1 1 1] Set Walk/Run Speed
  (set `CharacterMovementComponent.MaxWalkSpeed` 150.0 (`self.CharacterMovement`)))

(event `Run`
  ;[1 1 1] Set Walk/Run Speed
  (set `CharacterMovementComponent.MaxWalkSpeed` 400.0 (`self.CharacterMovement`)))

(event `self.ReceiveBeginPlay`
  (`/Engine/EditorBlueprintResources/ActorMacros.Switch Has Authority`
    (:`Authority`
      (`|ExecutionSequence`
        (:`then_0`
          (set `self.CurrentHealth` (`self.MaxHealth`)))))))

(event `Play_HADOUKEN_Anim`
  (`|PlayMontage` (`self.Mesh`) (`self.AM_Hadouken`) (`self.HadoukenPlayRate`)
    (:`OnCompleted`
      (bind _asenemy_c (cast `/Game/SmashBallsGame/Characters/Blueprints/Enemy_C` (`AIBlueprintHelperLibrary.GetAIController` self)))
      (`/Game/SmashBallsGame/Characters/Blueprints/Enemy_C.StopRotToPlayer` _asenemy_c))))

(event `SpawnHadouken`
  (bind _returnvalue (`self.GetTransform`))
  ;[1 1 1] Spawn Hadouken
  (`GameplayStatics.PlaySound2D` "/Game/Assets/Audio/Abilities/hadouken-sound-effect-NLoRkc06_Cue.hadouken-sound-effect-NLoRkc06_Cue")
  (bind _returnvalue_2 (`|SpawnActorFromClass` "/Game/SmashBallsGame/Weapons/Mortar/BPC_Proj_Hadouken.BPC_Proj_Hadouken_C" (`KismetMathLibrary.MakeTransform` (`KismetMathLibrary.MakeVector` (.x (.location _returnvalue)) (.y (.location _returnvalue)) (+ (.z (.location _returnvalue)) (`KismetMathLibrary.SelectFloat` 50.0 -25.0 (`KismetMathLibrary.RandomBool`)))) (.rotation _returnvalue) (.scale _returnvalue)) "AlwaysSpawn" "OverrideRootScale" self self))
  (`ProjectileMovementComponent.SetVelocityInLocalSpace` (`/Game/SmashBallsGame/Projectiles/Blueprints/BP_Projectile_Master.ProjectileMovement` _returnvalue_2) (400.0 0.0 0.0)))

(event `self.ReceiveAnyDamage`
  (params (Damage :type "Float (single-precision)") (DamageType :type "DamageType Object Reference") (InstigatedBy :type "Controller Object Reference") (DamageCauser :type "Actor Object Reference"))
  ;[1 0 0] Deal Damage & Kill Player
  (`KismetSystemLibrary.PrintString` (`KismetStringLibrary.Conv_DoubleToString` Damage))
  (bind _output_get (set `self.CurrentHealth` (`KismetMathLibrary.Clamp` (`KismetMathLibrary.FTrunc` (- (`KismetMathLibrary.Conv_IntToDouble` (`self.CurrentHealth`)) Damage)) 0 (`self.MaxHealth`))))
  (if (<= _output_get 0)
    (`/Engine/EditorBlueprintResources/StandardMacros.DoOnce` false
      (:`Completed`
        (set `self.IsDead?` true)
        (`self.Multicast_DeathSound`)
        (`self.K2_DestroyActor`)))))

(event `Multicast_DeathSound`
  ;[1 0 0] Deal Damage & Kill Player
  (`GameplayStatics.SpawnSoundAttached` (`self.DeathSound`) (`self.Mesh`)))

(event `self.PawnSensing.OnSeePawn`
  (params (Pawn :type "Pawn Object Reference"))
  (`KismetSystemLibrary.PrintString` (`KismetStringLibrary.Conv_VectorToString` (`self.K2_GetActorLocation` Pawn))))

(fn `UserConstructionScript`)