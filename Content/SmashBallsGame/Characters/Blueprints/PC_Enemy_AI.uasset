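; AI controller for enemies in SmashBallsGame that chases the player and performs a Hadouken attack once in range.
; A looping timer started on BeginPlay repeatedly issues AIMoveTo toward the player character with a wide acceptance radius.
; On a successful move it pauses the timer, tells the controlled Enemy to play its Hadouken animation, then resumes the chase after a short delay.
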(event `self.ReceiveBeginPlay`
  (`KismetSystemLibrary.K2_SetTimer` null "ChasePlayer" 0.5 true))

(event `ChasePlayer`
  (`|AIMoveTo` (`self.K2_GetPawn`) (0.0 0.0 0.0) (`GameplayStatics.GetPlayerCharacter` 0) 800.0
    (:`OnSuccess`
      (`KismetSystemLibrary.K2_PauseTimer` null "ChasePlayer")
      (bind _asenemy (cast `/Game/SmashBallsGame/Characters/Blueprints/Enemy` (`self.K2_GetPawn`)))
      (`/Game/SmashBallsGame/Characters/Blueprints/Enemy.Play_HADOUKEN_Anim` _asenemy)
      (`KismetSystemLibrary.Delay` 3.0)
      (`KismetSystemLibrary.K2_UnPauseTimer` null "ChasePlayer"))))

(fn `UserConstructionScript`)