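; ShootHadouken is a Behavior Tree task that makes an AI enemy fire a Hadouken attack.
; It casts the owner to Enemy_C and raises IsFiring on its BPEnemyRef enemy.
; It waits for the Hadouken animation's length, scaled by the enemy's play rate, then clears the flag and finishes successfully.
; The task only toggles the flag and times it, while a leftover player-death check is never run.
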(event `self.ReceiveExecute`
  (params (OwnerActor :type "Actor Object Reference"))
  (bind _asenemy_c (cast `/Game/SmashBallsGame/Characters/Blueprints/Enemy_C` OwnerActor))
  (bind _bp_enemyref (`/Game/SmashBallsGame/Characters/Blueprints/Enemy_C.BP_EnemyRef` _asenemy_c))
  (set `/Game/SmashBallsGame/Characters/Blueprints/Enemy_BP.IsFiring?` true _bp_enemyref)
  (bind _returnvalue (`AnimSequenceBase.GetPlayLength` (`self.AM_Hadouken`)))
  (`KismetSystemLibrary.Delay` (/ _returnvalue (`/Game/SmashBallsGame/Characters/Blueprints/Enemy_BP.HadoukenPlayRate` _bp_enemyref)))
  (set `/Game/SmashBallsGame/Characters/Blueprints/Enemy_BP.IsFiring?` false _bp_enemyref)
  (`self.FinishExecute` true))