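; Enemy_C is the AI controller for Enemy_BP, running the Enemy_BT behavior tree on possess.
; AI perception updates of BP_Character_Master actors write whether they are sensed to the enemy-visible Blackboard key.
; Helper events forward Walk/Run to the pawn and snap its yaw toward the player.
; Hadouken animation and perception-loop enemy-selection logic are left disconnected.
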(event `Walk`
  ;[1 1 1] Set Walk/Run Speed
  (`/Game/SmashBallsGame/Characters/Blueprints/Enemy_BP.Walk` (`self.BP_EnemyRef`)))

(event `Run`
  ;[1 1 1] Set Walk/Run Speed
  (`/Game/SmashBallsGame/Characters/Blueprints/Enemy_BP.Run` (`self.BP_EnemyRef`)))

(event `self.OnPossess`
  (params (PossessedPawn :type "Pawn Object Reference"))
  ;[1 1 1] Possess
  (bind _asenemy_bp (cast `/Game/SmashBallsGame/Characters/Blueprints/Enemy_BP` PossessedPawn))
  (set `self.BP_EnemyRef` _asenemy_bp)
  (`self.RunBehaviorTree` "/Game/SmashBallsGame/Characters/Blueprints/Enemy_BT.Enemy_BT"))

(event `self.AIPerception.OnTargetPerceptionUpdated`
  (params (Actor :type "Actor Object Reference") (Stimulus :type "AIStimulus Structure"))
  (cast `/Game/SmashBallsGame/Characters/Blueprints/BP_Character_Master` Actor)
  (`BlackboardComponent.SetValueAsBool` (`AIBlueprintHelperLibrary.GetBlackboard` null) (`self.BlackboardKeyIsEnemyVisible?`) (`.bSuccessfullySensed` (break `AIStimulus` Stimulus))))

(event `self.ReceiveBeginPlay`
  (bind _asbp_character_master (cast `/Game/SmashBallsGame/Characters/Blueprints/BP_Character_Master` (`GameplayStatics.GetPlayerCharacter` 0)))
  (set `self.BP_PlayerRef` _asbp_character_master))

(event `self.AIPerception.OnPerceptionUpdated`
  (params (UpdatedActors :type "Array of Actor Object Reference (by ref)")))

(event `StopRotToPlayer`
  (bind _returnvalue (`self.K2_GetPawn`))
  (bind (_returnvalue_roll _returnvalue_pitch) (`KismetMathLibrary.BreakRotator` (`self.K2_GetActorRotation` _returnvalue)))
  (bind (_returnvalue_roll_2 _returnvalue_pitch_2 _returnvalue_yaw) (`KismetMathLibrary.BreakRotator` (`KismetMathLibrary.FindLookAtRotation` (`self.K2_GetActorLocation` _returnvalue) (`self.K2_GetActorLocation` (`GameplayStatics.GetPlayerCharacter` 0)))))
  ;[1 1 1] Rotate to player when stopped
  (`self.K2_SetActorRotation` _returnvalue (`KismetMathLibrary.MakeRotator` _returnvalue_roll _returnvalue_pitch _returnvalue_yaw) false))

(fn `SetEnemy_BB`
  (params (NewEnemy :type "Actor Object Reference"))
  (if (!= NewEnemy (`self.Enemy`))
    (bind _output_get (set `self.Enemy` NewEnemy))
    (`BlackboardComponent.SetValueAsObject` (`AIBlueprintHelperLibrary.GetBlackboard` null) (`self.BlackboardKeyEnemy`) _output_get)))

(fn `UserConstructionScript`)