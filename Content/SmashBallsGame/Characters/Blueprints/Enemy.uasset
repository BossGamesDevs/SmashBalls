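; Enemy character Blueprint with a Hadouken attack that launches a mortar projectile.
; One custom event plays the Hadouken montage on the mesh; a separate event spawns the projectile, and nothing in this file calls either.
; The projectile spawns at the mesh transform, offset along world Y rather than its facing, with the enemy as owner and instigator.
; A forward and upward local-space velocity lobs it.
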(event `Play_HADOUKEN_Anim`
  (`|PlayMontage` (`self.Mesh`) "/Game/Assets/MyLittleMan/Animations/MyLittleMan_Anim_Tbag_HeroTPPTEST_001_HADOUKEN_Montage.MyLittleMan_Anim_Tbag_HeroTPPTEST_001_HADOUKEN_Montage"))

(event `SpawnHadouken`
  (bind _returnvalue (`SceneComponent.K2_GetComponentToWorld` (`self.Mesh`)))
  (bind _returnvalue_2 (`|SpawnActorFromClass` "/Game/SmashBallsGame/Weapons/Mortar/BPC_Proj_Mortar.BPC_Proj_Mortar_C" (`KismetMathLibrary.MakeTransform` (`KismetMathLibrary.MakeVector` (.x (.location _returnvalue)) (+ (.y (.location _returnvalue)) 250.0) (.z (.location _returnvalue))) (.rotation _returnvalue) (.scale _returnvalue)) "AlwaysSpawn" "OverrideRootScale" self self))
  (`ProjectileMovementComponent.SetVelocityInLocalSpace` (`/Game/SmashBallsGame/Projectiles/Blueprints/BP_Projectile_Master.ProjectileMovement` _returnvalue_2) (3500.0 0.0 1500.0)))

(fn `UserConstructionScript`)