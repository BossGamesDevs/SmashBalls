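; Master weapon Blueprint for networked shooting with single, auto, burst and multi fire, plus ammo, reload and configurable color.
; Mode macros gate a client-side muzzle sphere trace using player pawn 0, then pass the hit to the server.
; The server applies hitscan damage (headshot criticals or radial) or spawns a projectile, then handles ammo and cooldown.
; Multicasts play muzzle, surface-based impact and sound effects, with do-once guards for looping and multi-shot audio.
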(event `self.ReceiveBeginPlay`
  ;[1 0.6599 0] EventBeginPlay Set Ammo Counts
  (`/Engine/EditorBlueprintResources/ActorMacros.Switch Has Authority`
    (:`Authority`
      (set `self.CurrentMaxAmmo` (`self.MaxAmmo`))
      (set `self.CurrentAmmoInClip` (`self.MaxAmmoClipSize`)))))

(event `Client_OnWeaponFire`
  (switch `/Game/SmashBallsGame/Weapons/Blueprints/E_FiringModes` (`self.FiringMode`)
    (:`NewEnumerator0`
      (`self.SingleFireMode`
        (:`Out`
          _)))
    (:`NewEnumerator1`
      (`self.AutoFireMode` :!label _label
        (:`Out`
          _)))
    (:`NewEnumerator3`
      (`self.BurstFireMode`
        (:`Out`
          _)))
    (:`NewEnumerator4`
      (`self.MultiFireMode`
        (:`Out`
          _))))
  (bind (_hitresult _hit) (`self.WeaponSphereTrace`))
  (if (not (<= (`self.CurrentAmmoInClip`) 0))
    (`self.Server_ShootInfo` _hitresult _hit)
    (else
      ;[1 1 1] Stop Weapon Fire If Ammo Is = To Zero
      (`/Game/SmashBallsGame/Characters/Blueprints/BP_Character_Master.Server_StopWeaponFire` (cast `/Game/SmashBallsGame/Characters/Blueprints/BP_Character_Master` (`GameplayStatics.GetPlayerPawn` 0) :!pure true)))))

(event `Server_ShootInfo`
  (params (HitResult :type "HitResult Structure") (Hit :type Boolean))
  (set `self.IsCooldownActive?` true)
  (bind (_hitresultout _hitout) (`self.ShootInfo` HitResult Hit))
  (switch `/Game/SmashBallsGame/Weapons/Blueprints/E_FiringModes` (`self.FiringMode`)
    (:`NewEnumerator0`
      (`self.Multicast_SingleFireWeaponFX` _hitresultout _hitout :!label _label_2))
    (:`NewEnumerator1`
      (set `self.IsAutoFire?` true)
      (`self.Multicast_AutoFireWeaponFX` _hitresultout _hitout))
    (:`NewEnumerator3`
      (goto _label_2))
    (:`NewEnumerator4`
      (`self.Multicast_MultiFireWeaponFX` _hitresultout _hitout)
      (`/Engine/EditorBlueprintResources/StandardMacros.DoOnce` false :!label _label_3
        (:`Completed`
          _))))
  (`self.DecrementAmmo`)
  (`KismetSystemLibrary.PrintString` "Bang")
  (`KismetSystemLibrary.Delay` (`self.SingleFireCooldown`))
  (set `self.IsCooldownActive?` false))

(event `Client_OffWeaponFire`
  (`|ExecutionSequence`
    (:`then_0`
      (goto _label :!via `CloseGate`))
    (:`then_1`
      (`self.Server_OffWeaponFire`))))

(event `Server_OffWeaponFire`
  ;[1 1 1] Multicast OffWeaponFire
  (`|ExecutionSequence`
    (:`then_0`
      (goto _label_3 :!via `Reset`))
    (:`then_1`
      (`self.Multicast_OffWeaponFire`))))

(event `Multicast_SingleFireWeaponFX`
  (params (HitResult :type "HitResult Structure") (Hit :type Boolean))
  ;[1 1 1] SingleFire Weapon FX
  (`self.SingleFireWeaponFX` HitResult Hit))

(event `Server_OnWeaponReload`
  ;[1 1 1] Reload Weapon
  (`self.Multicast_ReloadSound`)
  (`KismetSystemLibrary.Delay` 2.0)
  (`self.ReloadAddAmmo`))

(event `Multicast_ReloadSound`
  ;[1 1 1] Reload Weapon
  (`GameplayStatics.SpawnSoundAttached` (`self.ReloadSound`) (`self.SK_WeaponMesh`)))

(event `Multicast_AutoFireWeaponFX`
  (params (HitResult :type "HitResult Structure") (Hit :type Boolean))
  ;[1 1 1] Autfire Weapon FX
  (`|ExecutionSequence`
    (:`then_0`
      (`self.AutoFireWeaponFX` HitResult Hit))
    (:`then_1`
      (`self.AutoFireSoundControl` :!label _label_4))))

(event `Multicast_OffWeaponFire`
  ;[1 1 1] Autfire Weapon FX
  (`|ExecutionSequence`
    (:`then_0`
      (goto _label_4 :!via `ResetDoOnce`))
    (:`then_1`
      (goto _label_4 :!via `FadeOut`))
    (:`then_2`
      (goto _label_5 :!via `ResetDoOnce`))))

(event `Multicast_MultiFireWeaponFX`
  (params (HitResult :type "HitResult Structure") (Hit :type Boolean))
  ;[1 1 1] MultiFire Weapon FX
  (`|ExecutionSequence`
    (:`then_0`
      (`self.MultiFireWeaponFX` HitResult Hit))
    (:`then_1`
      (`self.MultiFireReset` :!label _label_5))))

(fn `AutoFireWeaponFX`
  (params (HitResult :type "HitResult Structure") (Hit :type Boolean))
  (bind (_bblockinghit _binitialoverlap _time _distance _location _impactpoint _normal _impactnormal _physmat) (`GameplayStatics.BreakHitResult` HitResult))
  (bind _surfacetype (`PhysicalMaterial.SurfaceType` _physmat))
  (`GameplayStatics.SpawnEmitterAttached` (`self.MuzzleFlashPS`) (`self.SK_WeaponMesh`) (`self.MuzzleSocketName`))
  (if (`self.IsHitScan?`)
    (if Hit
      (`GameplayStatics.PlaySoundAtLocation` (select `EPhysicalSurface` _surfacetype :`SurfaceType_Default` (`self.DefaultBulletImpactSound`) :`SurfaceType1` (`self.PlayerBulletImpactSound`) :!type "SoundBase Object Reference") _impactpoint)
      (`GameplayStatics.SpawnEmitterAtLocation` (select `EPhysicalSurface` _surfacetype :`SurfaceType_Default` (`self.DefaultImpactPS`) :`SurfaceType1` (`self.PlayerImpactPS`)) _impactpoint (`KismetMathLibrary.MakeRotFromZ` _impactnormal)))))

(fn `DecrementAmmo`
  (set `self.CurrentAmmoInClip` (`KismetMathLibrary.Clamp` (- (`self.CurrentAmmoInClip`) 1) 0 (`self.MaxAmmoClipSize`))))

(fn `MultiFireWeaponFX`
  (params (HitResult :type "HitResult Structure") (Hit :type Boolean))
  (bind (_bblockinghit _binitialoverlap _time _distance _location _impactpoint _normal _impactnormal _physmat) (`GameplayStatics.BreakHitResult` HitResult))
  (bind _surfacetype (`PhysicalMaterial.SurfaceType` _physmat))
  (if (`self.IsHitScan?`)
    (if Hit
      (`GameplayStatics.PlaySoundAtLocation` (select `EPhysicalSurface` _surfacetype :`SurfaceType_Default` (`self.DefaultBulletImpactSound`) :`SurfaceType1` (`self.PlayerBulletImpactSound`) :!type "SoundBase Object Reference") _impactpoint)
      (`GameplayStatics.SpawnEmitterAtLocation` (select `EPhysicalSurface` _surfacetype :`SurfaceType_Default` (`self.DefaultImpactPS`) :`SurfaceType1` (`self.PlayerImpactPS`)) _impactpoint (`KismetMathLibrary.MakeRotFromZ` _impactnormal)))))

(fn `ReloadAddAmmo`
  (`/Engine/EditorBlueprintResources/ActorMacros.Switch Has Authority`
    (:`Authority`
      (set `self.AmmoNeededForReload` (- (`self.MaxAmmoClipSize`) (`self.CurrentAmmoInClip`)))
      (if (<= (`self.CurrentMaxAmmo`) (`self.AmmoNeededForReload`))
        (set `self.CurrentAmmoInClip` (+ (`self.CurrentAmmoInClip`) (`self.CurrentMaxAmmo`)))
        (set `self.CurrentMaxAmmo` 0)
        (else
          (set `self.CurrentMaxAmmo` (- (`self.CurrentMaxAmmo`) (`self.AmmoNeededForReload`)))
          (set `self.CurrentAmmoInClip` (`self.MaxAmmoClipSize`)))))))

(fn `ShootInfo`
  (params (HitResult :type "HitResult Structure (by ref)") (Hit :type Boolean))
  (returns (HitResultOut :type "HitResult Structure") (HitOut :type Boolean))
  (bind (_bblockinghit _binitialoverlap _time _distance _location _impactpoint _normal _impactnormal _physmat _hitactor _hitcomponent _hitbonename _hititem _faceindex _tracestart _traceend) (`GameplayStatics.BreakHitResult` HitResult))
  (bind _damage (`self.Damage`))
  (bind _returnvalue (`SceneComponent.GetSocketLocation` (`self.SK_WeaponMesh`) (`self.MuzzleSocketName`)))
  (if (`self.IsHitScan?`)
    (switch `/Game/SmashBallsGame/Weapons/Blueprints/E_DamageTypes` (`self.DamageType`)
      (:`NewEnumerator0`
        (if (`self.HasCriticalDamage?`)
          (switch `name` _hitbonename
            (:`Default`
              (`GameplayStatics.ApplyDamage` _hitactor (`KismetMathLibrary.Conv_IntToDouble` _damage) (`self.GetInstigatorController`) self :!label _label))
            (:`head`
              (`GameplayStatics.ApplyDamage` _hitactor (`KismetMathLibrary.Conv_IntToDouble` (* _damage (`self.CriticalMultiplier`))) (`self.GetInstigatorController`) self)))
          (else
            (goto _label))))
      (:`NewEnumerator1`
        (`GameplayStatics.ApplyRadialDamage` :`BaseDamage` (`KismetMathLibrary.Conv_IntToDouble` (`self.Damage`)) :`Origin` _impactpoint :`DamageRadius` (`self.DamageRadius`) :`DamageCauser` self :`InstigatedByController` (`self.GetInstigatorController`))))
    (else
      (`|SpawnActorFromClass` (`self.Projectile`) (`KismetMathLibrary.MakeTransform` _returnvalue (`KismetMathLibrary.FindLookAtRotation` _returnvalue (`KismetMathLibrary.SelectVector` _impactpoint _traceend Hit))) "AlwaysSpawn" "OverrideRootScale" (`self.GetOwner`) (`self.GetInstigator`))))
  (return HitResult Hit))

(fn `SingleFireWeaponFX`
  (params (HitResult :type "HitResult Structure") (Hit :type Boolean))
  (bind (_bblockinghit _binitialoverlap _time _distance _location _impactpoint _normal _impactnormal _physmat) (`GameplayStatics.BreakHitResult` HitResult))
  (bind _sk_weaponmesh (`self.SK_WeaponMesh`))
  (bind _surfacetype (`PhysicalMaterial.SurfaceType` _physmat))
  (`GameplayStatics.SpawnSoundAttached` (`self.SingleFireSound`) _sk_weaponmesh)
  (`GameplayStatics.SpawnEmitterAttached` (`self.MuzzleFlashPS`) _sk_weaponmesh (`self.MuzzleSocketName`))
  (if (`self.IsHitScan?`)
    (if Hit
      (`GameplayStatics.PlaySoundAtLocation` (select `EPhysicalSurface` _surfacetype :`SurfaceType_Default` (`self.DefaultBulletImpactSound`) :`SurfaceType1` (`self.PlayerBulletImpactSound`) :!type "SoundBase Object Reference") _impactpoint)
      (`GameplayStatics.SpawnEmitterAtLocation` (select `EPhysicalSurface` _surfacetype :`SurfaceType_Default` (`self.DefaultImpactPS`) :`SurfaceType1` (`self.PlayerImpactPS`)) _impactpoint (`KismetMathLibrary.MakeRotFromZ` _impactnormal)))))

(fn `UserConstructionScript`
  (bind _returnvalue (`PrimitiveComponent.CreateDynamicMaterialInstance` (`self.SK_WeaponMesh`) 0 "/Game/Assets/Weapons/Materials/M_Default_Weapon.M_Default_Weapon"))
  (`MaterialInstanceDynamic.SetVectorParameterValue` _returnvalue "Color" (`self.WeaponColor`))
  (bind _returnvalue_2 (`PrimitiveComponent.CreateDynamicMaterialInstance` (`self.SK_WeaponMesh`) 1 "/Game/Assets/Weapons/Materials/M_Default_Weapon.M_Default_Weapon"))
  (`MaterialInstanceDynamic.SetVectorParameterValue` _returnvalue_2 "Color" (`self.WeaponColor`)))

(fn `WeaponSphereTrace`
  (returns (HitResult :type "HitResult Structure") (Hit :type Boolean))
  (bind _asbp_character_master (cast `/Game/SmashBallsGame/Characters/Blueprints/BP_Character_Master` (`GameplayStatics.GetPlayerPawn` 0) :!pure true))
  (bind (_outhit _returnvalue) (`KismetSystemLibrary.SphereTraceSingle` (`SceneComponent.GetSocketLocation` (`self.SK_WeaponMesh`) (`self.MuzzleSocketName`)) (+ (`SceneComponent.K2_GetComponentLocation` (`/Game/SmashBallsGame/Characters/Blueprints/BP_Character_Master.TraceStartLocation` _asbp_character_master)) (* (`KismetMathLibrary.GetForwardVector` (`SceneComponent.GetSocketRotation` (`self.SK_WeaponMesh`) (`self.MuzzleSocketName`))) (`self.SphereTraceRange`))) (`self.SphereTraceRadius`) "TraceTypeQuery1" false (`|MakeArray` _asbp_character_master :!type "Actor Object Reference") "ForDuration"))
  (return _outhit _returnvalue))